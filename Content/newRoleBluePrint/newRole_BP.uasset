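; newRole_BP is a player character Blueprint handling movement, camera look and a dance emote.
; Axis inputs move the character relative to control yaw and drive controller pitch and yaw, while Left Shift switches walk speed between walking and sprinting.
; F plays the dancing montage on the mesh, and Tick stops it once the character's velocity shows it is moving.
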(event `InputAxis|MoveForward`
  (params (AxisValue :type "Float (single-precision)"))
  (bind (_returnvalue_roll _returnvalue_pitch _returnvalue_yaw) (`KismetMathLibrary.BreakRotator` (`self.GetControlRotation`)))
  ;[1 1 1] 角色位移和动画播放
  (`self.AddMovementInput` (`KismetMathLibrary.GetForwardVector` (`KismetMathLibrary.MakeRotator` 0.0 0.0 _returnvalue_yaw)) AxisValue))

(event `InputAxis|Turn`
  (params (AxisValue :type "Float (single-precision)"))
  ;[1 1 1] 角色位移和动画播放
  (`self.AddControllerYawInput` AxisValue))

(event `InputAxis|MoveRight`
  (params (AxisValue :type "Float (single-precision)"))
  (bind (_returnvalue_roll _returnvalue_pitch _returnvalue_yaw) (`KismetMathLibrary.BreakRotator` (`self.GetControlRotation`)))
  ;[1 1 1] 角色位移和动画播放
  (`self.AddMovementInput` (`KismetMathLibrary.GetRightVector` (`KismetMathLibrary.MakeRotator` 0.0 0.0 _returnvalue_yaw)) AxisValue))

(event `InputAxis|LookUp`
  (params (AxisValue :type "Float (single-precision)"))
  ;[1 1 1] 角色位移和动画播放
  (`self.AddControllerPitchInput` AxisValue))

(event `Key|LeftShift`
  (params (Key :type "Key Structure"))
  (bind _charactermovement (`self.CharacterMovement`))
  (:`Pressed`
    (set `CharacterMovementComponent.MaxWalkSpeed` 550.0 _charactermovement))
  (:`Released`
    (set `CharacterMovementComponent.MaxWalkSpeed` 150.0 _charactermovement)))

(event `Key|F`
  (params (Key :type "Key Structure"))
  ;[1 1 1] 蒙太奇操作
  (:`Pressed`
    (`AnimInstance.Montage_Play` (`SkeletalMeshComponent.GetAnimInstance` (`self.Mesh`)) "/Game/NEWROLE/DancingMontage.DancingMontage" 1.0 "MontageLength" 0.0 true)))

(event `self.ReceiveTick`
  (params (DeltaSeconds :type "Float (single-precision)"))
  ;[1 1 1] 蒙太奇操作
  (if (>= (`KismetMathLibrary.VSize` (`self.GetVelocity`)) 1.0)
    (`self.StopAnimMontage` "/Game/NEWROLE/DancingMontage.DancingMontage")))

(fn `UserConstructionScript`)